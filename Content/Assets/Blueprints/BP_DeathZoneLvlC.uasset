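; Spike death zone that reacts when a BP_Char overlaps its collision component.
; With a checkpoint set on the character, it moves player 0's character to the stored respawn transform.
; Otherwise it triggers the character's damage system, plays a death sound, then after a short delay shows the Level 3 death menu with the cursor visible and calls DisableInput on itself.
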(event OnComponentBeginOverlap(CollisionComponent)
  (params (OverlappedComponent :type Primitive%20Component%20Object%20Reference) (OtherActor :type Actor%20Object%20Reference) (OtherComp :type Primitive%20Component%20Object%20Reference) (OtherBodyIndex :type Integer) (bFromSweep :type Boolean) (SweepResult :type Hit%20Result%20Structure%20%28by%20ref%29))
  (bind _returnvalue (Game|GetPlayerController 0))
  ;[1 1 1] Plays sound and opens death menu when player comes in contack with spikes
  (bind _ascharacter (Utilities|Casting|CastToCharacter OtherActor))
  (bind _asbp_char (Utilities|Casting|CastToBP_Char _ascharacter))
  (if (Variables|/Game/Assets/Blueprints/BP_Char.BP_Char_C|GetCheckpoint _asbp_char)
    ;;[1 1 1] Sends the player to the checkpoint
    (Transformation|SetActorTransform (Game|GetPlayerCharacter 0) (Variables|/Game/Assets/Blueprints/BP_Char.BP_Char_C|GetrespawnTransform _asbp_char))
    (else
      (Default|DamageSystem _asbp_char true)
      (Audio|PlaySound2D "/Game/Assets/Sounds/S_DeathAudio.S_DeathAudio")
      (Utilities|FlowControl|Delay 0.3)
      (bind _returnvalue_2 (UserInterface|CreateWidget "/Game/Assets/Blueprints/W_DeathMenuLvl3.W_DeathMenuLvl3_C"))
      (UserInterface|Viewport|AddtoViewport _returnvalue_2 0)
      (Class|WidgetBlueprintLibrary|SetFocustoGameViewport)
      (Variables|/Script/Engine.PlayerController|SetbShowMouseCursor _returnvalue true)
      (Input|DisableInput _returnvalue))))

(fn ConstructionScript)