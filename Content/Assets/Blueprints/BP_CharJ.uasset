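; Side-scrolling Paper2D player character with run, jump, slide and death animations.
; Input, landing and death set an animation state that UpdateAnimation maps to flipbooks every Tick, choosing run or idle by speed.
; Tick also turns the controller to face travel and, once DamageSystem sets Dead, stops the sprite and disables input.
; Footsteps play on flipbook frames from the movement axis event; BoxJ block-spawning code is disconnected.
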(event Custom|UpdateAnimation
  (bind _sprite (Variables|Default|GetSprite))
  ;[1 1 1] Handle Animation
  (switch Utilities|FlowControl|Switch|SwitchonCharacter_states (Variables|Default|GetAmimate_states)
    (:NewEnumerator0
      (Sprite|SetFlipbook _sprite (select (> (Math|Vector|VectorLength (Transformation|GetVelocity)) 0.0) "/Game/Assets/Character/A_Run.A_Run" "/Game/Assets/Character/A_Idle.A_Idle") :!label _label))
    (:NewEnumerator1
      (goto _label))
    (:NewEnumerator4
      (Sprite|SetFlipbook _sprite "/Game/Assets/Character/A_Slide.A_Slide"))
    (:NewEnumerator5
      (Sprite|SetFlipbook _sprite "/Game/Assets/Character/A_Jump.A_Jump"))
    (:NewEnumerator6
      (Sprite|SetFlipbook _sprite "/Game/Assets/Character/A_Dead.A_Dead"))
    (:NewEnumerator7
      (Sprite|SetFlipbook _sprite "/Game/Assets/Character/A_Slide.A_Slide"))))

(event Custom|DamageSystem
  (params (Dmg :type Boolean))
  ;[1 1 1] Death system
  (Variables|Default|SetDead Dmg))

(event EventBeginPlay
  (Utilities|FlowControl|Sequence
    (:then_0
      (Class|ActorComponent|SetIsReplicated (Variables|Default|GetSprite) true))))

(event EventOnLanded
  (params (Hit :type Hit%20Result%20Structure%20%28by%20ref%29))
  ;[1 1 1] Handle Jump
  (if (not (Variables|Default|GetDead))
    (Audio|PlaySoundatLocation "/Game/Assets/Sounds/Landing_Cue.Landing_Cue" (Transformation|GetActorLocation))
    (Variables|Default|SetAmimate_states "NewEnumerator0")
    (CallFunction|UpdateAnimation)))

(event EventTick
  (params (DeltaSeconds :type Float%20%28single-precision%29))
  ;[1 1 1] Tick - Updates animation
  (CallFunction|UpdateAnimation)
  (Math|Float|CompareFloat (.X (Math|Vector|BreakVector (Variables|/Script/Engine.MovementComponent|GetVelocity (Pawn|GetMovementComponent)))) 0.0
    (:>
      (Pawn|SetControlRotation (Pawn|GetController) (Math|Rotator|MakeRotator 0.0 0.0 0.0) :!label _label))
    (:==
      (if (Variables|Default|GetbisMovingRight)
        (goto _label)
        (else
          (Pawn|SetControlRotation (Pawn|GetController) (Math|Rotator|MakeRotator 0.0 0.0 1.8e+02) :!label _label_2))))
    (:<
      (goto _label_2)))
  ;[1 1 1] Sets death animation
  (if (Variables|Default|GetDead)
    (Variables|Default|SetAmimate_states "NewEnumerator6")
    (Utilities|FlowControl|Sequence
      (:then_1
        (Utilities|FlowControl|Delay 0.3)
        (Audio|Components|Audio|Stop (Variables|Default|GetSprite)))
      (:then_2
        (Input|DisableInput 0)))))

(event Input|ActionEvents|InputActionPickUp
  (params (Key :type Key%20Structure :default "AnyKey"))
  ;[1 1 1] Spawn 2 blocks mechanic on k press each spawn deletes previous block
)

(event Input|ActionEvents|InputActionJump
  (params (Key :type Key%20Structure :default "AnyKey"))
  ;[1 1 1] Handle Jump
  (:Pressed
    (Character|Jump)
    (Variables|Default|SetAmimate_states "NewEnumerator5")
    (CallFunction|UpdateAnimation))
  (:Released
    (Character|StopJumping)))

(event Input|AxisEvents|InputAxisMoveRight
  (params (AxisValue :type Float%20%28single-precision%29))
  (bind _sprite (Variables|Default|GetSprite))
  (bind _returnvalue (Class|PaperFlipbookComponent|GetPlaybackPositioninFrames _sprite))
  ;[1 1 1] Handle movement
  (if (> AxisValue 0.0)
    (Variables|Default|SetbisMovingRight true)
    (elif (< AxisValue 0.0)
      (Variables|Default|SetbisMovingRight false)))
  (Pawn|Input|AddMovementInput "1.000000, 0, 0" AxisValue false)
  (if (Variables|Default|GetbisMovingRight)
    _
    (else
      _))
  (if (or (== _returnvalue 4) (== _returnvalue 9))
    (Audio|PlaySoundatLocation "/Game/Assets/Sounds/268758__deleted-user-5093904__footsteps_Cue.268758__deleted-user-5093904__footsteps_Cue" "0, 0, 0")))

(event Input|KeyboardEvents|S
  (params (Key :type Key%20Structure :default "AnyKey"))
  (bind _returnvalue (Game|GetPlayerCharacter 0))
  (bind _returnvalue_2 (Transformation|GetVelocity _returnvalue))
  (bind _x (Math|Vector|BreakVector _returnvalue_2))
  ;[1 1 1] Slide animation mechanic on S key press
  (:Pressed
    (if (> _x 0.0)
      (Development|PrintString (Utilities|String|ToString(Float) _x))
      (Variables|Default|SetAmimate_states "NewEnumerator4" :!label _label)
      (CallFunction|UpdateAnimation :!label _label_2)
      (elif (< _x 0.0)
        (Development|PrintString (Utilities|String|ToString(Float) _x))
        (goto _label))))
  (:Released
    (Variables|Default|SetAmimate_states "NewEnumerator0")
    (goto _label_2)))

(event Input|TouchEvents|InputTouch
  (params (Location :type Vector) (FingerIndex :type ETouchIndex%20Enum))
  ;[1 1 1] Handle Jump
  (:Pressed
    (Character|Jump)
    (Variables|Default|SetAmimate_states "NewEnumerator5")
    (CallFunction|UpdateAnimation))
  (:Released
    (Character|StopJumping)))

(fn ConstructionScript)