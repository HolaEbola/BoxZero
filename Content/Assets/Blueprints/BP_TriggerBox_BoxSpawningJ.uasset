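; Trigger box that lets the player spawn BP_Box actors while standing inside it.
; Overlap by a PaperCharacter enables the trigger's input and prints a prompt to press E, and end overlap disables input again.
; Each SpawnBlock press spawns a scaled box at a fixed world X offset from the trigger, nudged to avoid collisions or skipped if still blocked.
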(event OnComponentEndOverlap(CollisionComponent)
  (params (OverlappedComponent :type Primitive%20Component%20Object%20Reference) (OtherActor :type Actor%20Object%20Reference) (OtherComp :type Primitive%20Component%20Object%20Reference) (OtherBodyIndex :type Integer))
  ;[1 1 1] Checks if player is inside the trigger
  (Utilities|Casting|CastToPaperCharacter OtherActor)
  (Input|DisableInput (Game|GetPlayerController 0)))

(event OnComponentBeginOverlap(CollisionComponent)
  (params (OverlappedComponent :type Primitive%20Component%20Object%20Reference) (OtherActor :type Actor%20Object%20Reference) (OtherComp :type Primitive%20Component%20Object%20Reference) (OtherBodyIndex :type Integer) (bFromSweep :type Boolean) (SweepResult :type Hit%20Result%20Structure%20%28by%20ref%29))
  ;[1 1 1] Checks if player is inside the trigger
  (Utilities|Casting|CastToPaperCharacter OtherActor)
  (Input|EnableInput (Game|GetPlayerController 0))
  (Development|PrintText "Click E to spawn boxes"))

(event EventBeginPlay)

(event Collision|EventActorBeginOverlap
  (params (OtherActor :type Actor%20Object%20Reference)))

(event EventTick
  (params (DeltaSeconds :type Float%20%28single-precision%29)))

(event Input|ActionEvents|InputActionSpawnBlock
  (params (Key :type Key%20Structure :default "AnyKey"))
  ;[1 1 1] Spawn block after pressing E
  (:Pressed
    (Game|SpawnActorfromClass "/Game/Assets/Blueprints/BP_Box.BP_Box_C" (Math|Transform|MakeTransform (Math|Transform|TransformLocation (Math|Transform|MakeTransform "-100.000000,0.000000,0.000000") (Transformation|GetActorLocation)) "0, 0, 0" "2.200000,1.000000,2.290000") "AdjustIfPossibleButDontSpawnIfColliding" 0 0)))

(fn ConstructionScript)