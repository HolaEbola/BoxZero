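; BP_SpeedTriggerJ is a trigger volume meant to give speed to the BP_CharJ character.
; When a PaperCharacter begins overlapping its collision, it overwrites the capsule's physics linear velocity with a small +X vector, then a weaker one when the overlap ends.
; The velocity always goes to the first BP_CharJ found through GetAllActorsOfClass, whichever PaperCharacter triggered the overlap.
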(event OnComponentBeginOverlap(CollisionComponent)
  (params (OverlappedComponent :type Primitive%20Component%20Object%20Reference) (OtherActor :type Actor%20Object%20Reference) (OtherComp :type Primitive%20Component%20Object%20Reference) (OtherBodyIndex :type Integer) (bFromSweep :type Boolean) (SweepResult :type Hit%20Result%20Structure%20%28by%20ref%29))
  ;[1 1 1] Gives speed
  (Utilities|Casting|CastToPaperCharacter OtherActor)
  (bind _outactors (Actor|GetAllActorsOfClass "/Game/Assets/Blueprints/BP_CharJ.BP_CharJ_C"))
  (Class|PrimitiveComponent|SetAllPhysicsLinearVelocity (Variables|/Script/Engine.Character|GetCapsuleComponent (Utilities|Array|Get(acopy) _outactors)) "5.000000, 0, 0" false))

(event OnComponentEndOverlap(CollisionComponent)
  (params (OverlappedComponent :type Primitive%20Component%20Object%20Reference) (OtherActor :type Actor%20Object%20Reference) (OtherComp :type Primitive%20Component%20Object%20Reference) (OtherBodyIndex :type Integer))
  ;[1 1 1] Gives speed
  (Utilities|Casting|CastToPaperCharacter OtherActor)
  (bind _outactors (Actor|GetAllActorsOfClass "/Game/Assets/Blueprints/BP_CharJ.BP_CharJ_C"))
  (Class|PrimitiveComponent|SetAllPhysicsLinearVelocity (Variables|/Script/Engine.Character|GetCapsuleComponent (Utilities|Array|Get(acopy) _outactors)) "1.000000, 0, 0" false))

(event EventBeginPlay)

(event EventTick
  (params (DeltaSeconds :type Float%20%28single-precision%29)))

(fn ConstructionScript)