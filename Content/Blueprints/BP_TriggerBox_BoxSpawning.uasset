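; A trigger box that lets a Paper2D character respawn a Box by pressing E while inside it.
; Overlap begin enables input for player 0 and prints a prompt, and overlap end disables input.
; Pressing E destroys the first Box found in the level, and releasing E spawns a new one above the trigger, adjusting for collisions or skipping the spawn if blocked.
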(event OnComponentEndOverlap(CollisionComponent)
  (params (OverlappedComponent :type Primitive%20Component%20Object%20Reference) (OtherActor :type Actor%20Object%20Reference) (OtherComp :type Primitive%20Component%20Object%20Reference) (OtherBodyIndex :type Integer))
  ;[1 1 1] Checks if player is inside the trigger
  (Utilities|Casting|CastToPaperCharacter OtherActor)
  (Input|DisableInput (Game|GetPlayerController 0)))

(event OnComponentBeginOverlap(CollisionComponent)
  (params (OverlappedComponent :type Primitive%20Component%20Object%20Reference) (OtherActor :type Actor%20Object%20Reference) (OtherComp :type Primitive%20Component%20Object%20Reference) (OtherBodyIndex :type Integer) (bFromSweep :type Boolean) (SweepResult :type Hit%20Result%20Structure%20%28by%20ref%29))
  ;[1 1 1] Checks if player is inside the trigger
  (Utilities|Casting|CastToPaperCharacter OtherActor)
  (Input|EnableInput (Game|GetPlayerController 0))
  (Development|PrintString "Press E to spawn"))

(event EventBeginPlay)

(event Collision|EventActorBeginOverlap
  (params (OtherActor :type Actor%20Object%20Reference)))

(event EventTick
  (params (DeltaSeconds :type Float%20%28single-precision%29)))

(event Input|KeyboardEvents|E
  (params (Key :type Key%20Structure :default "AnyKey"))
  ;[1 1 1] Spawn block after pressing E
  (:Pressed
    (bind _outactors (Actor|GetAllActorsOfClass "/Game/Blueprints/box.Box_C"))
    (Actor|DestroyActor (Utilities|Array|Get(acopy) _outactors)))
  (:Released
    (Game|SpawnActorfromClass "/Game/Blueprints/box.Box_C" (Math|Transform|MakeTransform (Math|Transform|TransformLocation (Math|Transform|MakeTransform "0.000000,0.000000,200.000000") (Transformation|GetActorLocation)) "0, 0, 0" "1.000000,1.000000,1.000000") "AdjustIfPossibleButDontSpawnIfColliding" 0 0)))

(fn ConstructionScript)